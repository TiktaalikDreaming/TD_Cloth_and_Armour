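; Placeable shield decoration that displays the owning clan's emblem and can only be placed by clan members.
; A dynamic material on the static mesh copies emblem and background textures and tints from the guild's emblem material.
; Server and client refresh it through GameState emblem signals, with clients requesting a sync once owner ID and character are available.
; Tick acts as a retry, toggled off once the emblem texture applies.
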(event Custom|CharacterReady
  (bind _asconan_character (Utilities|Casting|CastToConanCharacter (Game|GetPlayerCharacter 0))
    (:then
      (Class|ConanCharacter|ServerSyncClanEmblemDatawithClient _asconan_character (Variables|Default|GetOwnerUniqueID))
      (EventDispatchers|BindEventtoSignalGuildEmblemUpdated (stale EventBeginPlay _asconan_game_state) (delegate Custom|EmblemUpdated)))
    (:CastFailed
      (bind _asconan_player_controller (Utilities|Casting|CastToConanPlayerController (Game|GetPlayerController 0)))
      (EventDispatchers|BindEventtoSignalCharacterReadyClient _asconan_player_controller (delegate Custom|CharacterReady)))))

(event Custom|OnGuildEmblemDataLoaded
  (params (GuildId :type Unique%20ID%20Object%20Reference))
  (if (== GuildId (Variables|Default|GetOwnerUniqueID))
    (bind _returnvalue (Class|Guild|GetGuildEmblem self GuildId))
    (CallFunction|SetEmblemMaterialParameters _returnvalue (Variables|Default|GetEmblemMaterial))))

(event Custom|OnServerEmblemDataLoaded
  (params (GuildId :type Unique%20ID%20Object%20Reference))
  (if (== GuildId (Variables|Default|GetOwnerUniqueID))
    (bind _returnvalue (Class|Guild|GetGuildEmblem self GuildId))
    (CallFunction|CreateDynamicMaterial)
    (CallFunction|SetEmblemMaterialParameters _returnvalue (Variables|Default|GetEmblemMaterial))))

(event Custom|OnReceivedOwnerUniqueID
  (bind _owneruniqueid (Variables|Default|GetOwnerUniqueID))
  (bind _asconan_game_state (Utilities|Casting|CastToConanGameState (Game|GetGameState)))
  (bind _returnvalue (Class|Guild|GetGuildEmblem self _owneruniqueid))
  (if (Utilities|IsValid _returnvalue)
    (CallFunction|SetEmblemMaterialParameters _returnvalue (Variables|Default|GetEmblemMaterial))
    (else
      (EventDispatchers|BindEventtoSignalonGuildEmblemDataLoaded _asconan_game_state (delegate Custom|OnGuildEmblemDataLoaded))))
  (bind _asconan_character (Utilities|Casting|CastToConanCharacter (Game|GetPlayerCharacter 0))
    (:then
      (Class|ConanCharacter|ServerSyncClanEmblemDatawithClient _asconan_character _owneruniqueid)
      (EventDispatchers|BindEventtoSignalGuildEmblemUpdated (stale EventBeginPlay _asconan_game_state) (delegate Custom|EmblemUpdated)))
    (:CastFailed
      (bind _asconan_player_controller (Utilities|Casting|CastToConanPlayerController (Game|GetPlayerController 0)))
      (EventDispatchers|BindEventtoSignalCharacterReadyClient _asconan_player_controller (delegate Custom|CharacterReady)))))

(event Custom|EmblemUpdated
  (params (GuildId :type Unique%20ID%20Object%20Reference))
  (if (== GuildId (Variables|Default|GetOwnerUniqueID))
    (bind _returnvalue (Class|Guild|GetGuildEmblem self GuildId))
    (CallFunction|SetEmblemMaterialParameters _returnvalue (Variables|Default|GetEmblemMaterial))))

(event EventBeginPlay
  (|CallParentFunction)
  (if (Networking|IsServer)
    (bind _asconan_game_state (Utilities|Casting|CastToConanGameState (Game|GetGameState)))
    (EventDispatchers|BindEventtoSignalonGuildEmblemDataLoaded _asconan_game_state (delegate Custom|OnServerEmblemDataLoaded))
    (EventDispatchers|BindEventtoSignalGuildEmblemUpdated _asconan_game_state (delegate Custom|EmblemUpdated))
    (bind _returnvalue (Class|Guild|GetGuildEmblem self (Variables|Default|GetOwnerUniqueID)))
    (if (Utilities|IsValid _returnvalue)
      (CallFunction|CreateDynamicMaterial)
      (CallFunction|SetEmblemMaterialParameters _returnvalue (Variables|Default|GetEmblemMaterial)))
    (else
      (bind _asconan_game_state_2 (Utilities|Casting|CastToConanGameState (Game|GetGameState)))
      (CallFunction|CreateDynamicMaterial)
      (EventDispatchers|BindEventtoSignalReceivedOwnerUniqueID (delegate Custom|OnReceivedOwnerUniqueID)))))

(event EventTick
  (params (DeltaSeconds :type Float%20%28single-precision%29))
  (bind _returnvalue (Class|Guild|GetGuildEmblem self (Variables|Default|GetOwnerUniqueID)))
  (CallFunction|SetEmblemMaterialParameters _returnvalue (Variables|Default|GetEmblemMaterial)))

(fn ConstructionScript
  (|CallParentFunction))

(fn CanbePlaced
  (params (AttachTo :type Buildable%20Base%20Object%20Reference) (InstanceIndex :type Integer))
  (bind (_failedmessage _returnvalue) (|CallParentFunction AttachTo InstanceIndex))
  (if (Utilities|Enum|Equal(Enum) _returnvalue "Success")
    (if (Networking|IsServer)
      (bind _asconan_game_state (Utilities|Casting|CastToConanGameState (Game|GetGameState))
        (:then
          (bind _returnvalue_2 (Class|ConanGameState|GetServerGuildfromId _asconan_game_state (Variables|Default|GetOwnerUniqueID)))
          (if (Utilities|IsValid _returnvalue_2)
            (return "" "Success")
            (else
              _)))
        (:CastFailed
          _))
      (else
        (bind _asconan_player_controller (Utilities|Casting|CastToConanPlayerController (Game|GetPlayerController 0))
          (:then
            (if (Utilities|IsValid (Class|ConanCharacter|GetGuild (Class|ConanPlayerController|GetConanCharacter _asconan_player_controller)))
              (return "" "Success")
              (else
                _)))
          (:CastFailed
            _))))
    (return (Utilities|String|ToString(Text) (Variables|Default|GetCannotPlaceMessage)) "Fail_NotMemberOfClan")
    (else
      (return _failedmessage _returnvalue))))

(fn SetEmblemMaterialParameters
  (params (GuildEmblem :type Material%20Instance%20Dynamic%20Object%20Reference) (ItemMaterial :type Material%20Instance%20Dynamic%20Object%20Reference))
  (if (and (Utilities|IsValid GuildEmblem) (Utilities|IsValid ItemMaterial))
    (bind _returnvalue (Rendering|Material|GetTextureParameterValue GuildEmblem "Emblem" :!class /Script/Engine.MaterialInstanceDynamic))
    (if (Utilities|IsValid _returnvalue)
      (Rendering|Material|SetTextureParameterValue ItemMaterial "Emblem" _returnvalue)
      (bind _returnvalue_2 (Rendering|Material|GetTextureParameterValue GuildEmblem "Background" :!class /Script/Engine.MaterialInstanceDynamic))
      (Rendering|Material|SetTextureParameterValue ItemMaterial "Background" _returnvalue_2)
      (bind _returnvalue_3 (Rendering|Material|GetVectorParameterValue GuildEmblem "Emblemtint" :!class /Script/Engine.MaterialInstanceDynamic))
      (Rendering|Material|SetVectorParameterValue ItemMaterial "Emblemtint" _returnvalue_3 :!class /Script/Engine.MaterialInstanceDynamic)
      (bind _returnvalue_4 (Rendering|Material|GetVectorParameterValue GuildEmblem "Backgroundtint" :!class /Script/Engine.MaterialInstanceDynamic))
      (Rendering|Material|SetVectorParameterValue ItemMaterial "Backgroundtint" _returnvalue_4 :!class /Script/Engine.MaterialInstanceDynamic)
      (Actor|Tick|SetActorTickEnabled false)
      (else
        (Actor|Tick|SetActorTickEnabled true :!label _label)))
    (else
      (goto _label))))

(fn CreateDynamicMaterial
  (bind _staticmesh (Variables|Default|GetStaticMesh))
  (bind _returnvalue (Rendering|Material|CreateDynamicMaterialInstance (Rendering|Material|GetMaterial _staticmesh (Variables|Default|GetEmblemMaterialIndex)) :!class /Script/Engine.KismetMaterialLibrary))
  (bind _output_get (Variables|Default|SetEmblemMaterial _returnvalue))
  (Rendering|Material|SetMaterial _staticmesh (Variables|Default|GetEmblemMaterialIndex) _output_get))